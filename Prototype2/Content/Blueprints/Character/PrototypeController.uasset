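; Player controller for PrototypeCharacter, handling movement, look, a grappling hook, a gravity gun and level restart after success.
; Holding right mouse runs timer-driven traces that grab light objects with a runtime-added PhysicsHandle and reel them closer.
; Left mouse throws the held object or fires the grapple.
; Tick extends the cable to the hit point, then pulls the player via repeated LaunchCharacter calls until jump or a new shot cancels it.
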(event `StopGrapple`
  (bind _grappleline (`/Game/Blueprints/Character/PrototypeCharacter.GrappleLine` (`self.CharacterPawn`)))
  (set `self.GrappleHooked?` false)
  (set `self.HookMoveFinish` false)
  (`SceneComponent.SetVisibility` _grappleline false false)
  (`SceneComponent.K2_SetWorldLocation` _grappleline (0.0 0.0 0.0) false false))

(event `RayTracePickup`
  (bind _characterpawn (`self.CharacterPawn`))
  (bind _characterpawn_2 (`self.CharacterPawn`))
  (bind _characterpawn_3 (`self.CharacterPawn`))
  (bind _camera (`/Game/Blueprints/Character/PrototypeCharacter.Camera` _characterpawn_3))
  (bind _beamps (`/Game/Blueprints/Character/PrototypeCharacter.BeamPS` (`self.CharacterPawn`)))
  ;[1 1 1] Basic Gravity Gun
  (bind (_outhit _returnvalue) (`KismetSystemLibrary.LineTraceSingleForObjects` (`SceneComponent.K2_GetComponentLocation` (`/Game/Blueprints/Character/PrototypeCharacter.FirePoint` _characterpawn_3)) (+ (`SceneComponent.K2_GetComponentLocation` _camera) (* (`SceneComponent.GetForwardVector` _camera) (`self.PickupDistance`))) (`self.PhysicsObjectTypes`)))
  (bind (_bblockinghit _binitialoverlap _time _location _impactpoint _normal _impactnormal _physmat _hitactor _hitcomponent) (`GameplayStatics.BreakHitResult` _outhit))
  (bind _output_get (set `self.PhysicsItemDistance` (`KismetMathLibrary.VSize` (- (`self.K2_GetActorLocation` _characterpawn) _location))))
  (set `self.PhysicsItemRotation` (`self.K2_GetActorRotation` _characterpawn))
  (if _returnvalue
    (if (< (`PrimitiveComponent.GetMass` _hitcomponent) (`self.MaxLiftWeight`))
      (`ActorComponent.Activate` _beamps false)
      (`ParticleSystemComponent.SetBeamTargetPoint` _beamps 0 _location 0)
      (`KismetSystemLibrary.K2_ClearAndInvalidateTimerHandle` (stale `InputAction|RightMouse` _returnvalue))
      (set `self.PickupDistance` _output_get)
      (bind _returnvalue_2 (`AddComponent|NODE_AddPhysicsHandleComponent-0` :`self` _characterpawn_2 :`RelativeTransform` (`self.GetTransform` _characterpawn_2)))
      (bind _output_get_2 (set `self.PhysicsHandle` _returnvalue_2))
      (set `self.PhysicsObject` _hitcomponent)
      (`PhysicsHandleComponent.GrabComponentAtLocation` _output_get_2 _hitcomponent "None" _location)
      (`PrimitiveComponent.SetCollisionResponseToChannel` _hitcomponent "ECC_Pawn" "ECR_Ignore")
      (bind _returnvalue_3 (`KismetSystemLibrary.K2_SetTimerDelegate` (delegate `UpdatePhysicObjDist`) 0.01 true))
      (set `self.PhysObjectUpdateTimer` _returnvalue_3))))

(event `UpdatePhysicObjDist`
  (bind _characterpawn (`self.CharacterPawn`))
  (bind _returnvalue (`Pawn.GetControlRotation` _characterpawn))
  ;[1 1 1] Basic Gravity Gun
  (if (> (`self.PickupDistance`) 300.0)
    (set `self.PickupDistance` (- (`self.PickupDistance`) 5.0)))
  (bind _output_get (set `self.HandleLocation` (+ (+ (`self.K2_GetActorLocation` _characterpawn) (* (`KismetMathLibrary.GetForwardVector` _returnvalue) (`self.PickupDistance`))) (0.0 0.0 100.0))))
  (`PhysicsHandleComponent.SetTargetLocationAndRotation` (`self.PhysicsHandle`) _output_get _returnvalue))

(event `EndPickup`
  (bind _physicshandle (`self.PhysicsHandle`))
  (bind _asprimitive_component (cast `PrimitiveComponent` (`self.PhysicsObject`) :!pure true))
  ;[1 1 1] Basic Gravity Gun
  (`/Engine/EditorBlueprintResources/StandardMacros.IsValid` _physicshandle
    (:`Is Valid`
      (`PhysicsHandleComponent.ReleaseComponent` _physicshandle)
      (`/Engine/EditorBlueprintResources/StandardMacros.IsValid` _asprimitive_component
        (:`Is Valid`
          (`PrimitiveComponent.SetCollisionResponseToChannel` _asprimitive_component "ECC_Pawn" "ECR_Block" :!label _label)
          (`ActorComponent.Deactivate` (`/Game/Blueprints/Character/PrototypeCharacter.BeamPS` (`self.CharacterPawn`)))
          (set `self.PickupDistance` 2000.0)
          (set `self.PhysicsHandleActive?` false)
          (`KismetSystemLibrary.K2_ClearAndInvalidateTimerHandle` (`self.PhysObjectUpdateTimer`)))))))

(event `InputAction|RightMouse`
  (params (Key :type "Key Structure"))
  ;[1 1 1] Basic Gravity Gun
  (:`Pressed`
    (set `self.PhysicsHandleActive?` true)
    (bind _returnvalue (`KismetSystemLibrary.K2_SetTimerDelegate` (delegate `RayTracePickup`) 0.01 true)))
  (:`Released`
    (set `self.PhysicsHandleActive?` false)
    (set `self.PickupDistance` 1500.0)
    (`KismetSystemLibrary.K2_ClearAndInvalidateTimerHandle` _returnvalue)
    (`self.EndPickup`)))

(event `self.ReceiveTick`
  (params (DeltaSeconds :type "Float (single-precision)"))
  (bind _grappleline (`/Game/Blueprints/Character/PrototypeCharacter.GrappleLine` (`self.CharacterPawn`)))
  ;[1 1 1] TICK
  (if (`self.GrappleHooked?`)
    (if (`self.HookMoveFinish`)
      (`self.MoveGrappledPlayer`)
      (`SceneComponent.K2_SetWorldLocation` _grappleline (`KismetMathLibrary.VInterpTo` (`SceneComponent.K2_GetComponentLocation` _grappleline) (`self.GrappleHookLocation`) (`GameplayStatics.GetWorldDeltaSeconds`) (`self.GrapplePlayerSpeed`)) false false)
      (else
        (bind _locationreached_ (`self.MoveRope`))
        (set `self.HookMoveFinish` _locationreached_)))))

(event `InputAction|LeftMouse`
  (params (Key :type "Key Structure"))
  (bind _characterpawn (`self.CharacterPawn`))
  (bind _asprimitive_component (cast `PrimitiveComponent` (`self.PhysicsObject`) :!pure true))
  (bind _camera (`/Game/Blueprints/Character/PrototypeCharacter.Camera` _characterpawn))
  ;[1 1 1] Basic Gravity Gun
  (:`Pressed`
    (if (`self.PhysicsHandleActive?`)
      (`/Engine/EditorBlueprintResources/StandardMacros.IsValid` _asprimitive_component
        (:`Is Valid`
          (`PhysicsHandleComponent.ReleaseComponent` (`self.PhysicsHandle`))
          (`PrimitiveComponent.AddImpulse` _asprimitive_component (* (`SceneComponent.GetForwardVector` (`/Game/Blueprints/Character/PrototypeCharacter.Camera` (`self.CharacterPawn`))) (`self.ThrowForce`)) "None" true)
          (goto _label)))
      (else
        (if (`self.GrappleHooked?`)
          (`self.StopGrapple`))
        (bind (_outhit _returnvalue) (`KismetSystemLibrary.LineTraceSingleForObjects` (`SceneComponent.K2_GetComponentLocation` (`/Game/Blueprints/Character/PrototypeCharacter.FirePoint` _characterpawn)) (+ (`SceneComponent.K2_GetComponentLocation` _camera) (* (`SceneComponent.GetForwardVector` _camera) (`self.GrappleDistance`))) (`|MakeArray` "ObjectTypeQuery1" "ObjectTypeQuery2" :!type "EObjectTypeQuery Enum")))
        (if _returnvalue
          (set `self.GrappleHooked?` true)
          (set `self.GrappleHookLocation` (`.Location` (`GameplayStatics.BreakHitResult` _outhit)))
          (else
            (`self.StopGrapple`)))))))

(event `SetupGrapple`
  (bind _grappleline (`/Game/Blueprints/Character/PrototypeCharacter.GrappleLine` (`self.CharacterPawn`)))
  ;[1 1 1] Grapple Setup
  (`SceneComponent.SetVisibility` _grappleline false false)
  (set `CableComponent.CableLength` 0.0 _grappleline)
  (set `CableComponent.CableWidth` 15.0 _grappleline)
  (set `CableComponent.EndLocation` (0.0 0.0 0.0) _grappleline))

(event `self.ReceiveBeginPlay`
  (bind _asprototype_character (cast `/Game/Blueprints/Character/PrototypeCharacter` (`self.K2_GetPawn`) :!pure true))
  ;[1 1 1] BeginPlay
  (`/Engine/EditorBlueprintResources/StandardMacros.IsValid` _asprototype_character
    (:`Is Valid`
      (set `self.CharacterPawn` _asprototype_character)
      (`self.SetupGrapple`))))

(event `CustomDisableMovement`
  ;[1 1 1] DisableMovement
  (set `self.DisableMovement?` true))

(event `InputAction|Reset`
  (params (Key :type "Key Structure"))
  (bind (_asprototype_game_mode_1 _bsuccess) (cast `/Game/Blueprints/Gamemode/PrototypeGameMode1` (`GameplayStatics.GetGameMode`) :!pure true))
  ;[1 1 1] ResetLevel
  (:`Pressed`
    (if _bsuccess
      (`/Game/Blueprints/Gamemode/PrototypeGameMode1.RestartLevel` _asprototype_game_mode_1))))

(event `InputAxis|LeftRightMovement`
  (params (AxisValue :type "Float (single-precision)"))
  (bind _returnvalue (`self.K2_GetPawn`))
  ;[1 1 1] WASD Movement
  (if (`self.DisableMovement?`)
    _
    (elif (not (`self.GrappleHooked?`))
      (`Pawn.AddMovementInput` _returnvalue (`KismetMathLibrary.GetRightVector` (`KismetMathLibrary.MakeRotator` 0.0 0.0 (.yaw (`Pawn.GetControlRotation` _returnvalue)))) AxisValue false))))

(event `InputAxis|ForwardBackMovement`
  (params (AxisValue :type "Float (single-precision)"))
  (bind _returnvalue (`self.K2_GetPawn`))
  ;[1 1 1] WASD Movement
  (if (`self.DisableMovement?`)
    _
    (elif (not (`self.GrappleHooked?`))
      (`Pawn.AddMovementInput` _returnvalue (`KismetMathLibrary.GetForwardVector` (`KismetMathLibrary.MakeRotator` 0.0 0.0 (.yaw (`Pawn.GetControlRotation` _returnvalue)))) AxisValue false))))

(event `InputAxis|Turn`
  (params (AxisValue :type "Float (single-precision)"))
  ;[1 1 1] Mouse Movement
  (if (not (`self.DisableMovement?`))
    (`self.AddYawInput` AxisValue)))

(event `InputAxis|LookUp`
  (params (AxisValue :type "Float (single-precision)"))
  ;[1 1 1] Mouse Movement
  (if (not (`self.DisableMovement?`))
    (`self.AddPitchInput` AxisValue)))

(event `InputAction|Jump`
  (params (Key :type "Key Structure"))
  (bind _characterpawn (`self.CharacterPawn`))
  ;[1 1 1] Jump & Crouch
  (:`Pressed`
    (if (`self.GrappleHooked?`)
      (`Character.LaunchCharacter` _characterpawn (0.0 0.0 500.0) false false))
    (`self.StopGrapple`)
    (`Character.Jump` _characterpawn)))

(event `InputAction|Crouch`
  (params (Key :type "Key Structure"))
  (bind _characterpawn (`self.CharacterPawn`))
  ;[1 1 1] Jump & Crouch
  (:`Pressed`
    (`Character.Crouch` _characterpawn))
  (:`Released`
    (`Character.UnCrouch` _characterpawn)))

(fn `MoveGrappledPlayer`
  (bind _characterpawn (`self.CharacterPawn`))
  (`Character.LaunchCharacter` _characterpawn (* (- (`self.GrappleHookLocation`) (`self.K2_GetActorLocation` _characterpawn)) (* (`GameplayStatics.GetWorldDeltaSeconds`) (`self.GrapplePlayerSpeed`))) true true))

(fn `MoveRope`
  (returns (`LocationReached?` :type Boolean))
  (bind _grapplehooklocation (`self.GrappleHookLocation`))
  (bind _grappleline (`/Game/Blueprints/Character/PrototypeCharacter.GrappleLine` (`self.CharacterPawn`)))
  (bind _returnvalue (`SceneComponent.K2_GetComponentLocation` _grappleline))
  (`SceneComponent.SetVisibility` _grappleline true false)
  (if (<= (`KismetMathLibrary.VSize` (- _returnvalue _grapplehooklocation)) 100.0)
    (return true)
    (else
      (`SceneComponent.K2_SetWorldLocation` _grappleline (`KismetMathLibrary.VInterpTo` _returnvalue _grapplehooklocation (`GameplayStatics.GetWorldDeltaSeconds`) (`self.GrappleRopeSpeed`)) false false)
      (return false))))

(fn `UpdatePhysObjectLocation`
  (bind _characterpawn (`self.CharacterPawn`))
  (bind _returnvalue (`Pawn.GetControlRotation` _characterpawn))
  (bind _output_get (set `self.HandleLocation` (+ (+ (`self.K2_GetActorLocation` _characterpawn) (* (`KismetMathLibrary.GetForwardVector` _returnvalue) (`self.PickupDistance`))) (0.0 0.0 500.0))))
  (`PhysicsHandleComponent.SetTargetLocationAndRotation` (`self.PhysicsHandle`) _output_get _returnvalue))

(fn `UserConstructionScript`)