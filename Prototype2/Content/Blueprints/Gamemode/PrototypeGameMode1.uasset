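; Game mode that handles the end of a game and level restarts for the prototype.
; On BeginPlay it binds handlers to the EndGame and RestartLevel dispatchers.
; Game end shows the EndScreen widget, focuses it after a zero-length delay, shows the mouse cursor and disables movement through PrototypeController.
; Restart reopens the current level by name.
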(event `self.ReceiveBeginPlay`
  (add `self.EndGame` (delegate `GameEnd`))
  (add `self.RestartLevel` (delegate `GM_RestartLevel`)))

(event `GM_RestartLevel`
  (bind _returnvalue (`GameplayStatics.GetCurrentLevelName` true))
  (`GameplayStatics.OpenLevel` (`KismetStringLibrary.Conv_StringToName` _returnvalue)))

(event `GameEnd`
  (bind _returnvalue (`GameplayStatics.GetPlayerController` 0))
  (bind (_asprototype_controller _bsuccess) (cast `/Game/Blueprints/Character/PrototypeController` _returnvalue :!pure true))
  (bind _returnvalue_2 (`|CreateWidget` "/Game/UI/EndScreen.EndScreen_C" _returnvalue))
  (`UserWidget.AddToViewport` _returnvalue_2 0)
  (`KismetSystemLibrary.Delay` 0.0)
  (`Widget.SetKeyboardFocus` _returnvalue_2)
  (set `PlayerController.bShowMouseCursor` true _returnvalue)
  (if _bsuccess
    (`/Game/Blueprints/Character/PrototypeController.CustomDisableMovement` _asprototype_controller)))

(fn `UserConstructionScript`)